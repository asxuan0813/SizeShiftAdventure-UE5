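; BP_SizeShiftPlayerController is the player controller that handles mouse input mode and pause menu toggling.
; On BeginPlay it sets game-only input and hides the cursor.
; Escape pauses the game with a newly created WBP_PauseMenu in Game and UI input mode with the cursor shown, or unpauses, removes the menu and restores game-only input with the cursor hidden.
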(event `self.ReceiveBeginPlay`
  (bind _returnvalue (`GameplayStatics.GetPlayerController` 0))
  (`WidgetBlueprintLibrary.SetInputMode_GameOnly` _returnvalue)
  (set `PlayerController.bShowMouseCursor` false _returnvalue))

(event `Key|Escape` :paused true
  (params (Key :type "Key Structure"))
  (bind _returnvalue (`GameplayStatics.GetPlayerController` 0))
  (bind _returnvalue_2 (`GameplayStatics.GetPlayerController` 0))
  (:`Pressed`
    (if (`GameplayStatics.IsGamePaused`)
      (`GameplayStatics.SetGamePaused` false)
      (`Widget.RemoveFromParent` (`self.PauseMenu`))
      (`WidgetBlueprintLibrary.SetInputMode_GameOnly` _returnvalue)
      (set `PlayerController.bShowMouseCursor` false _returnvalue)
      (else
        (bind _returnvalue_3 (`|CreateWidget` "/Game/UI/UI/WBP_PauseMenu.WBP_PauseMenu_C"))
        (bind _output_get (set `self.PauseMenu` _returnvalue_3))
        (`UserWidget.AddToViewport` _output_get 0)
        (`GameplayStatics.SetGamePaused` true)
        (`WidgetBlueprintLibrary.SetInputMode_GameAndUIEx` _returnvalue_2 _returnvalue_3)
        (set `PlayerController.bShowMouseCursor` true _returnvalue_2)))))

(fn `UserConstructionScript`)